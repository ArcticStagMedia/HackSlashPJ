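; Base pickup item that the archer player collects into the HUD inventory and uses to add Health, Energy and Mood.
; The Construction Script fills its inventory struct and sets the mesh from variables.
; A collection radius toggles the name widget and in-range flag, gating a handler bound to the player's PickupItem dispatcher.
; Collected items are hidden with collision off, not destroyed, and the struct's self-reference keeps UseAction on the actor.
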(event OnComponentEndOverlap(CollectionRadius)
  (params (OtherActor :type Actor%20Object%20Reference) (OtherComp :type Primitive%20Component%20Object%20Reference) (OtherBodyIndex :type Integer))
  ;[1 1 1] Trigger
  (Utilities|Casting|CastToArcherCharacter OtherActor)
  (Variables|/Game/UI/PickupText.PickupText_C|SetIsDisplayed? (Variables|Default|GetPickupTextWidget) "Hidden")
  (Variables|Default|SetIsInRange false))

(event OnComponentBeginOverlap(CollectionRadius)
  (params (OtherActor :type Actor%20Object%20Reference) (OtherComp :type Primitive%20Component%20Object%20Reference) (OtherBodyIndex :type Integer) (bFromSweep :type Boolean) (SweepResult :type Hit%20Result%20Structure%20%28by%20ref%29))
  ;[1 1 1] Trigger
  (Utilities|Casting|CastToArcherCharacter OtherActor)
  (Variables|/Game/UI/PickupText.PickupText_C|SetIsDisplayed? (Variables|Default|GetPickupTextWidget) "Visible")
  (Variables|Default|SetIsInRange true))

(event Custom|PickupItem_Event
  (bind _playercharacter (Variables|Default|GetPlayerCharacter))
  (bind _gamehudwidget (Variables|/Game/Character/Blueprints/ArcherCharacter.ArcherCharacter_C|GetGameHudWidget _playercharacter))
  ;[1 1 1] Pick up Item
  (if (and (Collision|GetActorEnableCollision) (Variables|Default|GetIsInRange))
    (Utilities|Array|Add (Variables|/Game/UI/GameHUD.GameHUD_C|GetInventory _gamehudwidget) (Variables|Default|GetItemInfo))
    (Rendering|SetActorHiddenInGame true)
    (Physics|SetSimulatePhysics (Variables|Default|GetPickup) false)
    (Collision|SetActorEnableCollision false)
    (Default|RefreshInventory _gamehudwidget)))

(event EventBeginPlay
  (bind _iteminfo (Variables|Default|GetItemInfo))
  ;[1 1 1] Event Begin Play
  (bind _aspickup_text (Utilities|Casting|CastToPickupText (UserInterface|GetUserWidgetObject (Variables|Default|GetDisplayPickupText))))
  (Variables|Default|SetPickupTextWidget _aspickup_text)
  (Variables|/Game/UI/PickupText.PickupText_C|SetPickupText _aspickup_text (.ItemName (Utilities|Struct|BreakInventoryStruct _iteminfo)))
  (Utilities|Struct|SetmembersinInventoryStruct _iteminfo self)
  (if (Utilities|IsValid (Variables|Default|GetPlayerCharacter))
    _
    (else
      (bind _asarcher_character (Utilities|Casting|CastToArcherCharacter (Game|GetPlayerCharacter 0)))
      (bind _output_get (Variables|Default|SetPlayerCharacter _asarcher_character))))
  (EventDispatchers|AssignPickupItem _output_get (delegate Custom|PickupItem_Event)))

(event EventUseAction
  (bind _playercharacter (Variables|Default|GetPlayerCharacter))
  (bind _gamehudwidget (Variables|/Game/Character/Blueprints/ArcherCharacter.ArcherCharacter_C|GetGameHudWidget _playercharacter))
  ;[1 1 1] Use Item
  (Variables|/Game/Character/Blueprints/ArcherCharacter.ArcherCharacter_C|SetHealth _playercharacter (+ (Variables|/Game/Character/Blueprints/ArcherCharacter.ArcherCharacter_C|GetHealth _playercharacter) (Variables|Default|GetAddHealth)))
  (Variables|/Game/Character/Blueprints/ArcherCharacter.ArcherCharacter_C|SetEnergy _playercharacter (+ (Variables|/Game/Character/Blueprints/ArcherCharacter.ArcherCharacter_C|GetEnergy _playercharacter) (Variables|Default|GetAddEnergy)))
  (Variables|/Game/Character/Blueprints/ArcherCharacter.ArcherCharacter_C|SetMood _playercharacter (+ (Variables|/Game/Character/Blueprints/ArcherCharacter.ArcherCharacter_C|GetMood _playercharacter) (Variables|Default|GetAddMood)))
  (Default|RefreshInventory _gamehudwidget)
  (Default|ActionComplete _gamehudwidget))

(fn ConstructionScript
  (Utilities|Struct|SetmembersinInventoryStruct (Variables|Default|GetItemInfo) self (Variables|Default|GetItemImage) (Variables|Default|GetItemName) (Variables|Default|GetActionText))
  (Components|StaticMesh|SetStaticMesh (Variables|Default|GetPickup) (Variables|Default|GetCustomMesh)))